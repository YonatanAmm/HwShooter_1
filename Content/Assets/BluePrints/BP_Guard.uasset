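; BP_Guard is an enemy AI that patrols between a target and its spawn point, detects the player and chases them, printing "Game Over" on reaching them.
; Tick drives a Patrol/Detection/Chase state machine from a range overlap and a head-pivot line trace, which latches line of sight and turns the guard toward the player.
; Chase heads back to spawn after a delay, then resumes patrol.
; DealDamage subtracts health, destroying the guard and calling EnemyFelled at zero.
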(event OnComponentBeginOverlap(Range)
  (params (OverlappedComponent :type Primitive%20Component%20Object%20Reference) (OtherActor :type Actor%20Object%20Reference) (OtherComp :type Primitive%20Component%20Object%20Reference) (OtherBodyIndex :type Integer) (bFromSweep :type Boolean) (SweepResult :type Hit%20Result%20Structure%20%28by%20ref%29))
  ;[0.2428 1 0.9002] On Enter/Exit Range
  (if (== OtherActor (Game|Player|GetPlayerPawn 0))
    (Variables|Default|SetInRange true)))

(event OnComponentEndOverlap(Range)
  (params (OverlappedComponent :type Primitive%20Component%20Object%20Reference) (OtherActor :type Actor%20Object%20Reference) (OtherComp :type Primitive%20Component%20Object%20Reference) (OtherBodyIndex :type Integer))
  ;[0.2428 1 0.9002] On Enter/Exit Range
  (if (== OtherActor (Game|Player|GetPlayerPawn 0))
    (Variables|Default|SetInRange false)))

(event Custom|StateCheck
  ;[1 1 1] State Check, Determins to which state do I want to get to
  (if (Math|Boolean|ANDBoolean (Variables|Default|GetInRange) (Variables|Default|GetInLoS) (Utilities|Enum|NotEqual(Enum) (Variables|Default|GetState) "NewEnumerator2"))
    (Variables|Default|SetState "NewEnumerator1")
    (Utilities|FlowControl|Delay 3.0)
    (if (and (Variables|Default|GetInRange) (Variables|Default|GetInLoS))
      (Variables|Default|SetState "NewEnumerator2")
      (else
        (Variables|Default|SetState "NewEnumerator0")))
    (elif (Utilities|Enum|NotEqual(Enum) (Variables|Default|GetState) "NewEnumerator2")
      (Variables|Default|SetState "NewEnumerator0"))))

(event Custom|ActOnState
  ;[1 0.6406 0.6406] State Mechine, Only enters the check when the desired state is different than the current one
  (if (Utilities|Enum|NotEqual(Enum) (Variables|Default|GetCurrentState) (Variables|Default|GetState))
    (switch Utilities|FlowControl|Switch|SwitchonE_States (Variables|Default|GetState)
      (:NewEnumerator0
        ;[1 0.6406 0.6406] Patrol State Logic
        (Variables|Default|SetCurrentState "NewEnumerator0")
        (AI|AIMoveTo self "0, 0, 0" (Variables|Default|GetTarget) 5.0 true :!label _label
          (:OnSuccess
            (AI|AIMoveTo self (Variables|Default|GetSpawnLocation) 0 5.0 true
              (:OnSuccess
                (goto _label))))))
      (:NewEnumerator1
        ;[1 0.6302 0.6302] Detection State Logic, look at player has the rotation to make it happen every tick
        (Variables|Default|SetCurrentState "NewEnumerator1")
        (AI|Navigation|StopMovement (Pawn|GetController self)))
      (:NewEnumerator2
        ;[1 0.651 0.651] Chase State Logic
        (Variables|Default|SetCurrentState "NewEnumerator2")
        (AI|AIMoveTo self "0, 0, 0" (Game|Player|GetPlayerPawn 0) 5.0 true
          (:then
            (Utilities|FlowControl|Delay 3.0)
            (AI|AIMoveTo self (Variables|Default|GetSpawnLocation) 0 5.0 false
              (:OnSuccess
                (Utilities|FlowControl|Delay 3.0)
                (Variables|Default|SetState "NewEnumerator0"))))
          (:OnSuccess
            (Development|PrintString "Game Over!!!" true true "(R=1.000000,G=0.000000,B=0.000000,A=1.000000)" 3e+01)))))))

(event EventBeginPlay
  ;[1 0.868 0.4896] Determins the spawn location to add it to the patrol path
  (Variables|Default|SetSpawnLocation (Transformation|GetActorLocation)))

(event EventTick
  (params (DeltaSeconds :type Float%20%28single-precision%29))
  ;[0.4582 1 0.5302] Event Tick, Determains which state should I be and act upon it when a change is needed
  (CallFunction|StateCheck)
  (CallFunction|ActonState)
  (if (Variables|Default|GetInRange)
    (CallFunction|LookatPlayer)
    (CallFunction|StateCheck)
    (else
      (CallFunction|StateCheck))))

(event EventDealDamage
  (params (DamageDone :type Float%20%28double-precision%29))
  ;[0.6885 0.4766 1] Damage Dealt Logic
  (Variables|Default|SetHealthPoints (- (Variables|Default|GetHealthPoints) DamageDone))
  (Development|PrintString (Utilities|String|Append "The damage done is: " (Utilities|String|ToString(Float) DamageDone) " Damage" "Hp left: " (Utilities|String|ToString(Float) (Variables|Default|GetHealthPoints))) true true "(R=0.000000,G=1.000000,B=0.098334,A=1.000000)" 5.0)
  (if (<= (Variables|Default|GetHealthPoints) 0.0)
    (Actor|DestroyActor)
    (Default|CallEnemyFelled)))

(fn ConstructionScript)

(fn LookatPlayer
  (bind _outhit (Collision|LineTraceByChannel (Transformation|GetWorldLocation (Variables|Default|GetHeadPivot)) (Transformation|GetActorLocation (Game|Player|GetPlayerPawn 0)) "TraceTypeQuery1" false 0 "Persistent"))
  (if (== (.HitActor (Collision|BreakHitResult _outhit)) (Game|GetPlayerCharacter 0))
    (Variables|Default|SetInLoS true)
    (Transformation|SetActorRotation (Math|Rotator|FindLookatRotation (Transformation|GetWorldLocation (Variables|Default|GetHeadPivot)) (Transformation|GetActorLocation (Game|Player|GetPlayerPawn 0))))))