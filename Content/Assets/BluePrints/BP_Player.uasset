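; Player Blueprint that fires, collects and cycles through weapons, keeping an ammo count for each.
; The held weapon is a child actor whose class changes on pickup or swap and is driven through message calls.
; Overlaps use interface checks to tell weapons from magazines, which add capped ammo to the matching weapon type.
; Parallel WepList and BulletNum arrays store inventory, saving and reloading counts as weapons change.
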(event Custom|Shoot
  ;[1 0.6042 0.6042] Shoot Logic
  (Class|BPIUseable|Attack(Message) (Variables|/Script/Engine.ChildActorComponent|GetChildActor (Variables|Default|GetWeapon%20Comp))))

(event Custom|SwapWeapons
  (bind _weapon_comp (Variables|Default|GetWeapon%20Comp))
  (bind _weapon_comp_2 (Variables|Default|GetWeapon%20Comp))
  (bind _childactor (Variables|/Script/Engine.ChildActorComponent|GetChildActor _weapon_comp_2))
  ;[0.5204 1 0.9801] Swap Weapon Through Tab Logic
  (if (Utilities|IsValid _childactor)
    (bind _ammo (Class|BPIUseable|ReloadAmmo(Message) _childactor))
    (Utilities|Array|SetArrayElem (Variables|Default|GetBulletNum) (Variables|Default|GetCurrentWeapon) _ammo))
  (Math|Integer|IncrementInt (Variables|Default|GetCurrentWeapon)
    (:%20%20
      (if (< (Variables|Default|GetCurrentWeapon) (Utilities|Array|Length (Variables|Default|GetWepList)))
        _
        (else
          (Variables|Default|SetCurrentWeapon 0)))
      (ChildActorComponent|SetChildActorClass _weapon_comp (Utilities|Array|Get(acopy) (Variables|Default|GetWepList) (Variables|Default|GetCurrentWeapon)))
      (Class|BPIUseable|Load(Message) (Variables|/Script/Engine.ChildActorComponent|GetChildActor _weapon_comp) (Utilities|Array|Get(acopy) (Variables|Default|GetBulletNum) (Variables|Default|GetCurrentWeapon))))))

(event Collision|EventActorBeginOverlap
  (params (OtherActor :type Actor%20Object%20Reference))
  (bind _weapon_comp (Variables|Default|GetWeapon%20Comp))
  (bind _weapon_comp_2 (Variables|Default|GetWeapon%20Comp))
  (bind _weplist (Variables|Default|GetWepList))
  (bind _bulletnum (Variables|Default|GetBulletNum))
  (bind _returnvalue (Utilities|Array|Length _weplist))
  (bind _childactor (Variables|/Script/Engine.ChildActorComponent|GetChildActor _weapon_comp))
  (bind _childactor_2 (Variables|/Script/Engine.ChildActorComponent|GetChildActor _weapon_comp_2))
  ;[0.5842 0.4927 1] Overlapping Logic Handler
  (if (Utilities|DoesObjectImplementInterface OtherActor "/Game/Assets/BluePrints/Interfaces/BPI_Collectiable.BPI_Collectiable_C")
    (if (Utilities|DoesObjectImplementInterface OtherActor "/Game/Assets/BluePrints/Interfaces/BPI_Useable.BPI_Useable_C")
      ;[0.4816 1 0.4595] Collecting A Weapon & Synch To Bullet Count Logic, could add more options on new overlaps if needed, for now we have just those two
      (if (Utilities|IsValid (Variables|/Script/Engine.ChildActorComponent|GetChildActor (Variables|Default|GetWeapon%20Comp)))
        (bind _ammo (Class|BPIUseable|ReloadAmmo(Message) (Variables|/Script/Engine.ChildActorComponent|GetChildActor (Variables|Default|GetWeapon%20Comp))))
        (Utilities|Array|SetArrayElem (Variables|Default|GetBulletNum) (Variables|Default|GetCurrentWeapon) _ammo))
      (ChildActorComponent|SetChildActorClass (Variables|Default|GetWeapon%20Comp) (Utilities|GetClass OtherActor))
      (bind _classtype (Class|BPICollectiable|OnCollectWeapon(Message) OtherActor))
      (bind _returnvalue_2 (Utilities|Array|AddUnique (Variables|Default|GetWepList) _classtype))
      (if (> _returnvalue_2 0)
        (Variables|Default|SetCurrentWeapon _returnvalue_2))
      (if (and (== _returnvalue 1) (!= (- _returnvalue 1) (Utilities|Array|Length (Variables|Default|GetBulletNum))))
        (Class|BPIUseable|Load(Message) _childactor_2 (Utilities|Array|Get(acopy) (Variables|Default|GetBulletNum) (Variables|Default|GetCurrentWeapon)))
        (else
          (Utilities|Array|AddUnique (Variables|Default|GetBulletNum) 0)
          (Class|BPIUseable|Load(Message) _childactor_2 5)))
      (Actor|DestroyActor OtherActor)
      (else
        ;[1 0.9211 0.5718] Collecting Mag & Bullet Managment Logic, placed the bullet managment here for modullar code, loading the specific instance with the information from bulletnum, and handles bullet managment logic in the weapon
        (bind (_bulletnum_2 _magtype) (Class|BPICollectiable|OnCollectMag(Message) OtherActor))
        (bind (_array_element _array_index) (Utilities|Array|ForEachLoopwithBreak (Variables|Default|GetWepList))
          (:LoopBody
            (if (== _magtype _array_element)
              (Utilities|Array|SetArrayElem _bulletnum _array_index (+ _bulletnum_2 (Utilities|Array|Get(acopy) _bulletnum _array_index)))
              (if (> (Utilities|Array|Get(acopy) _bulletnum _array_index) 50)
                (Utilities|Array|SetArrayElem (Variables|Default|GetBulletNum) _array_index 50)
                (Class|BPIUseable|Load(Message) _childactor 50)
                (else
                  (Class|BPIUseable|Load(Message) _childactor _bulletnum_2)))
              (Actor|DestroyActor OtherActor))))))))

(fn ConstructionScript)