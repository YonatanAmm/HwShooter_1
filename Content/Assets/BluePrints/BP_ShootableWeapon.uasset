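; Shootable weapon actor that fires physics-driven BP_Bullet projectiles while it has ammo.
; Attack spawns a scaled-down bullet at BulletSpawner, sets its damage by WeaponType (Rifle or Shotgun), launches it with a forward impulse and decrements Ammo.
; Load adds incoming ammo to the current count up to a fixed cap.
; Small functions expose the weapon class and current ammo, while OnCollectMag returns a zero bullet count.
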(event EventBeginPlay)

(event Collision|EventActorBeginOverlap
  (params (OtherActor :type Actor%20Object%20Reference)))

(event EventTick
  (params (DeltaSeconds :type Float%20%28single-precision%29)))

(event EventAttack
  (if (> (Variables|Default|GetAmmo) 0)
    (bind _returnvalue (Game|SpawnActorfromClass "/Game/Assets/BluePrints/BP_Bullet.BP_Bullet_C" (Math|Transform|MakeTransform (Transformation|GetWorldLocation (Variables|Default|GetBulletSpawner)) "0, 0, 0" "0.050000,0.050000,0.050000") "Undefined" "MultiplyWithRoot" 0 0))
    (switch Utilities|FlowControl|Switch|SwitchonE_WeaponType (Variables|Default|GetWeaponType)
      (:NewEnumerator0
        (Variables|/Game/Assets/BluePrints/BP_Bullet.BP_Bullet_C|SetDamage _returnvalue 1e+01))
      (:NewEnumerator1
        (Variables|/Game/Assets/BluePrints/BP_Bullet.BP_Bullet_C|SetDamage _returnvalue 1e+02)))
    (Physics|AddImpulse (Variables|/Game/Assets/BluePrints/BP_Bullet.BP_Bullet_C|GetSphere _returnvalue) (* (Math|Vector|GetForwardVector (Variables|Default|GetBulletSpawner)) 4e+02) "None" false)
    (Math|Integer|DecrementInt (Variables|Default|GetAmmo))
    (else
      (Development|PrintString "No Bullets Left!!"))))

(event EventLoad
  (params (CurrentAmmo :type Integer))
  ;[1 1 1] Load Bullet Info, loads when picked up/swapping weapon. Handles bullet managment in Attack logic
  (if (> (+ CurrentAmmo (Variables|Default|GetAmmo)) 50)
    (Variables|Default|SetAmmo 50)
    (else
      (Variables|Default|SetAmmo (+ CurrentAmmo (Variables|Default|GetAmmo))))))

(fn ConstructionScript)

(fn OnCollectMag
  (return 0 0))

(fn OnCollectWeapon
  (return (Utilities|GetClass self)))

(fn ReloadAmmo
  (return (Variables|Default|GetAmmo)))