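; GM_GameMode1 is a game mode that handles the win condition and ammo pickup spawning.
; On BeginPlay it binds every BP_Guard's EnemyFelled dispatcher to a counter event, which prints a win message once the count equals the guard total.
; The same per-guard loop scatters a batch of randomly chosen rifle or shotgun mags across hard-coded floor bounds, so pickup count scales with guard count.
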(event Custom|EnemyFelled_Event
  ;[0.9909 0.6084 1] Bind Guards To Death Event & Winning Logic, might have been an overkill, wanted to make stuff as general and modullar as I could
  (Math|Integer|IncrementInt (Variables|Default|GetCounter)
    (:%20%20
      (if (== (Variables|Default|GetCounter) (Utilities|Array|Length (Variables|Default|GetEnemies)))
        (Development|PrintString "You Have Won!!" true true "(R=1.000000,G=0.782915,B=0.000000,A=1.000000)" 3e+01)))))

(event EventBeginPlay
  ;[0.9909 0.6084 1] Bind Guards To Death Event & Winning Logic, might have been an overkill, wanted to make stuff as general and modullar as I could
  (bind _outactors (Actor|GetAllActorsOfClass "/Game/Assets/BluePrints/BP_Guard.BP_Guard_C"))
  (bind _output_get (Variables|Default|SetEnemies _outactors))
  (for _array_element _output_get
    (EventDispatchers|AssignEnemyFelled _array_element (delegate Custom|EnemyFelled_Event))
    ;[1 0.4638 0.5336] Spawn Mags Logic, based on the size of the "Floor" Asset
    (for _index (range 0 9)
      (bind _output_get_2 (Variables|Default|SetMag%20Spawn%20Location (Math|Vector|MakeVector (Math|Random|RandomFloatinRange -3.5e+03 3.5e+03) (Math|Random|RandomFloatinRange -3.5e+03 3.5e+03) 3e+01)))
      (if (== (Math|Random|RandomIntegerinRange 0 1) 0)
        (Game|SpawnActorfromClass "/Game/Assets/BluePrints/BP_RifleMag.BP_RifleMag_C" (Math|Transform|MakeTransform _output_get_2 "0, 0, 0" "2.000000,2.000000,2.000000") "AdjustIfPossibleButAlwaysSpawn" "MultiplyWithRoot" 0 0)
        (else
          (Game|SpawnActorfromClass "/Game/Assets/BluePrints/BP_ShotgunMag.BP_ShotgunMag_C" (Math|Transform|MakeTransform _output_get_2 "0, 0, 0" "2.000000,2.000000,2.000000") "AdjustIfPossibleButAlwaysSpawn" "MultiplyWithRoot" 0 0))))))

(event EventTick
  (params (DeltaSeconds :type Float%20%28single-precision%29)))

(fn ConstructionScript)